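; Charge-up plasma gun weapon: holding fire builds charge, and releasing fires one plasma projectile that carries the charge level.
; A looping timer created on BeginPlay stays paused until SFire, adding charge up to a cap while it runs.
; SStopFire pauses it, spawns the projectile at the muzzle along the holder's aim, then resets the charge.
; M_SetChargeMaterial lights five indicator meshes and updates the HUD ammo readout with non-zero charge.
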(event Custom|AddCharge
  (bind _output_get (Variables|Default|SetplasmaCharge (Math|Integer|Min(Integer) (+ (Variables|Default|GetplasmaCharge) 1) 5)))
  (CallFunction|MSetChargeMaterial _output_get))

(event Custom|M_SetChargeMaterial
  (params (Charge :type Integer))
  (if (!= Charge 0)
    (Rendering|Material|SetMaterial (Utilities|Select :Index Charge :Option%200 0 :Option%201 (Variables|Default|GetStaticMesh) :Option%202 (Variables|Default|GetStaticMesh1) :Option%203 (Variables|Default|GetStaticMesh2) :Option%204 (Variables|Default|GetStaticMesh3) :Option%205 (Variables|Default|GetStaticMesh4)) 0 "/Game/Items/Weapons/PlasmaGun/Materials/M_PlasmaChargeFull.M_PlasmaChargeFull")
    (Class|BPIPlayerHud|SetAmmoState(Message) (Variables|/Game/ThirdPerson/Blueprints/BP_ThirdPersonCharacter.BP_ThirdPersonCharacter_C|GetPlayerHud (Variables|Default|GetHoldingCharacter)) (Variables|Default|GetplasmaCharge) (Variables|Default|GetMaxAmmo))
    (else
      (Rendering|Material|SetMaterial (Variables|Default|GetStaticMesh) 0 "/Game/Items/Weapons/PlasmaGun/Materials/M_PlasmaChargeZero.M_PlasmaChargeZero"))))

(event EventBeginPlay
  (|CallParentFunction)
  (bind _returnvalue (Utilities|Time|SetTimerbyEvent (delegate Custom|AddCharge) 0.25 true))
  (bind _output_get (Variables|Default|SetchargeTimerHandle _returnvalue))
  (Utilities|Time|PauseTimerbyHandle _output_get))

(event Collision|EventActorBeginOverlap
  (params (OtherActor :type Actor%20Object%20Reference))
  (|CallParentFunction OtherActor) ; This node is disabled and will not be called.\nDrag off pins to build functionality.
)

(event EventTick
  (params (DeltaSeconds :type Float%20%28single-precision%29))
  (|CallParentFunction DeltaSeconds) ; This node is disabled and will not be called.\nDrag off pins to build functionality.
)

(event EventSFire
  (|CallParentFunction)
  (Utilities|Time|UnpauseTimerbyHandle (Variables|Default|GetchargeTimerHandle)))

(event EventSStopFire
  (|CallParentFunction)
  (Utilities|Time|PauseTimerbyHandle (Variables|Default|GetchargeTimerHandle))
  (if (> (Variables|Default|GetplasmaCharge) 0)
    (Game|SpawnActorfromClass "/Game/Items/Projectiles/BP_PlasmaProjectile.BP_PlasmaProjectile_C" (Math|Transform|MakeTransform (Transformation|GetWorldLocation (Variables|Default|GetMuzzle)) (Variables|/Game/ThirdPerson/Blueprints/BP_ThirdPersonCharacter.BP_ThirdPersonCharacter_C|GetAimRotation (Variables|Default|GetHoldingCharacter)) "1.000000,1.000000,1.000000") "AdjustIfPossibleButAlwaysSpawn" "MultiplyWithRoot" (Components|GetOwner) (Variables|Default|GetplasmaCharge) (Variables|Default|GetdamageType) 0)
    (Variables|Default|SetplasmaCharge 0)
    (CallFunction|MSetChargeMaterial)
    (CallFunction|Shot)))

(fn ConstructionScript
  (|CallParentFunction))

(fn OnRepPlasmaCharge)

(fn OnRepChargeTimerHandle)

(fn GetAmmoState
  (return (Variables|Default|GetplasmaCharge) (Variables|Default|GetMaxAmmo)))