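; Base weapon Blueprint that provides shared firing state and aim-point tracking, apparently for child weapons to extend.
; Tick line-traces forward from the muzzle on the Camera channel and caches the hit, exposed through GetLookingPointHit.
; StartFire and StopFire forward to S_-prefixed events that toggle IsFiring.
; Reload, the ammo getter and both OnRep handlers are empty or placeholder stubs.
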(event Custom|S_StopFire
  (Variables|Default|SetisFiring false))

(event Custom|S_Fire
  (Variables|Default|SetisFiring true))

(event Custom|S_Reload)

(event EventBeginPlay)

(event Collision|EventActorBeginOverlap
  (params (OtherActor :type Actor%20Object%20Reference)))

(event EventTick
  (params (DeltaSeconds :type Float%20%28single-precision%29))
  (bind _muzzle (Variables|Default|GetMuzzle))
  (bind _returnvalue (Transformation|GetWorldLocation _muzzle))
  (bind _outhit (Collision|LineTraceByChannel _returnvalue (+ _returnvalue (* (Math|Vector|GetForwardVector _muzzle) 5e+04)) "TraceTypeQuery2" false 0 "None"))
  (Variables|Default|SetweaponLookingPoint _outhit))

(event EventStopFire
  (CallFunction|SStopFire))

(event EventStartFire
  (CallFunction|SFire))

(fn ConstructionScript)

(fn OnRepIsFiring)

(fn OnRepWeaponIronsightHit)

(fn GetAmmoState
  (return 0 0))

(fn GetLookingPointHit
  (return (Variables|Default|GetweaponLookingPoint)))