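; Plasma projectile whose effect size, blast radius and damage scale with a Charge value.
; On BeginPlay it multiplies EmitterScale by Charge, which then sizes both the hit effects and the damage sphere.
; A blocking hit spawns effects, then the authority damages overlapped WorldDynamic and Pawn actors by BaseDamage times Charge.
; Both authority and remote branches then destroy the projectile.
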(event Custom|S_SetEmiterScale
  (Variables|Default|SetEmitterScale (* (Variables|Default|GetEmitterScale) (Variables|Default|Getcharge))))

(event EventBeginPlay
  (|CallParentFunction)
  (CallFunction|SSetEmiterScale))

(event Collision|EventActorBeginOverlap
  (params (OtherActor :type Actor%20Object%20Reference))
  (|CallParentFunction OtherActor) ; This node is disabled and will not be called.\nDrag off pins to build functionality.
)

(event EventTick
  (params (DeltaSeconds :type Float%20%28single-precision%29))
  (|CallParentFunction DeltaSeconds) ; This node is disabled and will not be called.\nDrag off pins to build functionality.
)

(event EventSProjectileHit
  (params (Hit :type Hit%20Result%20Structure%20%28by%20ref%29))
  (bind (_bblockinghit _binitialoverlap _time _distance _location _impactpoint _normal _impactnormal) (Collision|BreakHitResult Hit))
  (if _bblockinghit
    (CallFunction|MSpawnHitEffects _location _impactnormal (Variables|Default|GetEmitterScale))
    (Networking|SwitchHasAuthority
      (:Authority
        (bind _outactors (Collision|SphereOverlapActors _location (* (Math|Vector|VectorLength (Variables|Default|GetEmitterScale)) 5e+01) (Utilities|Array|MakeArray "ObjectTypeQuery2" "ObjectTypeQuery3") 0))
        (for _array_element _outactors
          (Game|Damage|ApplyDamage _array_element (* (Variables|Default|GetBase%20Damage) (Variables|Default|Getcharge)) 0 0 (Variables|Default|GetDamage%20Type%20Class)))
        (Actor|DestroyActor))
      (:Remote
        (Actor|DestroyActor)))))

(fn ConstructionScript
  (|CallParentFunction))

(fn OnRepCharge)