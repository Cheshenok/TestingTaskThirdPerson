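; Base projectile actor that damages what it hits, spawns an impact particle effect and destroys itself.
; Static mesh hits feed S_ProjectileHit, which on blocking hits applies damage only with authority, while both authority and remote branches spawn effects and destroy the actor.
; M_SpawnHitEffects spawns the pooled emitter aligned to the impact normal.
; OnRep handlers for damage, emitter template and scale are empty.
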(event OnComponentHit(StaticMesh)
  (params (HitComponent :type Primitive%20Component%20Object%20Reference) (OtherActor :type Actor%20Object%20Reference) (OtherComp :type Primitive%20Component%20Object%20Reference) (NormalImpulse :type Vector :default "0, 0, 0") (Hit :type Hit%20Result%20Structure%20%28by%20ref%29))
  (CallFunction|SProjectileHit Hit))

(event Custom|M_SpawnHitEffects
  (params (Location :type Vector) (ImpactNormal :type Vector) (Scale :type Vector))
  (Effects|SpawnEmitteratLocation (Variables|Default|GetEmitter%20Template) Location (Math|Conversions|RotationFromXVector ImpactNormal) Scale true "AutoRelease"))

(event Custom|S_ProjectileHit
  (params (Hit :type Hit%20Result%20Structure%20%28by%20ref%29))
  (bind (_bblockinghit _binitialoverlap _time _distance _location _impactpoint _normal _impactnormal _physmat _hitactor) (Collision|BreakHitResult Hit))
  (if _bblockinghit
    (Networking|SwitchHasAuthority
      (:Authority
        (Game|Damage|ApplyDamage _hitactor (Variables|Default|GetBase%20Damage) 0 0 (Variables|Default|GetDamage%20Type%20Class))
        (CallFunction|MSpawnHitEffects _impactpoint _impactnormal (Variables|Default|GetEmitterScale))
        (Actor|DestroyActor))
      (:Remote
        (CallFunction|MSpawnHitEffects _impactpoint _impactnormal (Variables|Default|GetEmitterScale))
        (Actor|DestroyActor)))))

(event EventBeginPlay)

(event Collision|EventActorBeginOverlap
  (params (OtherActor :type Actor%20Object%20Reference)))

(event EventTick
  (params (DeltaSeconds :type Float%20%28single-precision%29)))

(fn ConstructionScript)

(fn OnRepEmitterTemplate)

(fn OnRepEmitterScale)

(fn OnRepBaseDamage)